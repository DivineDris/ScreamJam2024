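; Base NPC character that shows a line of dialogue and turns to face the player when interacted with.
; OnInteract saves the starting rotation, prints PhraseText and runs a looping timer that eases yaw toward the player.
; After a delay, a second timer eases the NPC back to its original yaw, then IsReadyToTalk re-enables interaction.
; The construction script also sets SprintSpeed.
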(event `/Game/Systems/Interaction/BPI_Interactable.OnInteract`
  (params (IsPlayerOverlapping :type Boolean))
  (if (`self.IsReadyToTalk`)
    (set `self.IsReadyToTalk` false)
    (set `self.InitialRotation` (`self.K2_GetActorRotation`))
    (bind _returnvalue (`KismetSystemLibrary.K2_SetTimer` null "RotateToPlayer" 0.01 true))
    (set `self.TimerHandle` _returnvalue)
    (`KismetSystemLibrary.PrintText` (`self.PhraseText`) true true (struct :`R` 1.0 :`B` 0.090198 :`A` 1.0) 5.0)
    (`KismetSystemLibrary.Delay` 5.0)
    (`KismetSystemLibrary.K2_ClearAndInvalidateTimerHandle` (`self.TimerHandle`))
    (bind _returnvalue_2 (`KismetSystemLibrary.K2_SetTimer` null "RotateToInitialRotation" 0.03 true))
    (`KismetSystemLibrary.Delay` 3.0)
    (`KismetSystemLibrary.K2_ClearAndInvalidateTimerHandle` _returnvalue_2)
    (set `self.IsReadyToTalk` true)))

(fn `RotateToInitialRotation`
  (bind (_returnvalue_roll _returnvalue_pitch _returnvalue_yaw) (`KismetMathLibrary.BreakRotator` (`KismetMathLibrary.RInterpTo` (`self.K2_GetActorRotation`) (`self.InitialRotation`) (`GameplayStatics.GetWorldDeltaSeconds`) 3.0)))
  (`self.K2_SetActorRotation` (`KismetMathLibrary.MakeRotator` 0.0 0.0 _returnvalue_yaw)))

(fn `RotateToPlayer`
  (bind (_returnvalue_roll _returnvalue_pitch _returnvalue_yaw) (`KismetMathLibrary.BreakRotator` (`KismetMathLibrary.RInterpTo` (`self.K2_GetActorRotation`) (`KismetMathLibrary.FindLookAtRotation` (`self.K2_GetActorLocation`) (`self.K2_GetActorLocation` (`self.Player`))) (`GameplayStatics.GetWorldDeltaSeconds`) 3.0)))
  (set `self.Player` (`GameplayStatics.GetPlayerCharacter` 0))
  (`self.K2_SetActorRotation` (`KismetMathLibrary.MakeRotator` 0.0 0.0 _returnvalue_yaw)))

(fn `UserConstructionScript`
  (set `self.SprintSpeed` 700.0))