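; BP_ObjectiveTrigger tracks the remaining contamination objectives and unlocks the exit once none are left.
; On BeginPlay it sets the objective count from the number of actors tagged "contamination", and the first player overlap with its trigger prints that count.
; Each CollectObjective event decrements and prints the count; at zero it sets IsReadyToLeave on the first BP_OutsideDoor tagged "OutsideDoor".
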(event `self.ReceiveBeginPlay`
  (`self.Initialize`))

(event `self.Trigger.OnComponentBeginOverlap`
  (params (OverlappedComponent :type "PrimitiveComponent Object Reference") (OtherActor :type "Actor Object Reference") (OtherComp :type "PrimitiveComponent Object Reference") (OtherBodyIndex :type Integer) (bFromSweep :type Boolean) (SweepResult :type "HitResult Structure (by ref)"))
  (if (== OtherActor (`GameplayStatics.GetPlayerCharacter` 0))
    (`/Engine/EditorBlueprintResources/StandardMacros.DoOnce` false
      (:`Completed`
        (`KismetSystemLibrary.PrintString` (`KismetStringLibrary.Conv_IntToString` (`self.NumberOfObjectives`)))))))

(event `/Game/Systems/Objective/BPI_ObjectiveCollector.CollectObjective`
  (bind _numberofobjectives (`self.NumberOfObjectives`))
  (if (> _numberofobjectives 0) :!label _label
    (bind _output_get (set `self.NumberOfObjectives` (- _numberofobjectives 1)))
    (`KismetSystemLibrary.PrintString` (`KismetStringLibrary.Conv_IntToString` _output_get))
    (if (not (> (`self.NumberOfObjectives`) 0))
      (goto _label))
    (else
      (bind _outactors (`GameplayStatics.GetAllActorsOfClassWithTag` "/Game/Objects/Doors/BP_OutsideDoor.BP_OutsideDoor_C" "OutsideDoor"))
      (set `/Game/Objects/Doors/BP_OutsideDoor.IsReadyToLeave` true (`|GetArrayItem` _outactors)))))

(fn `Initialize`
  (bind _outactors (`GameplayStatics.GetAllActorsWithTag` "contamination"))
  (set `self.NumberOfObjectives` (`KismetArrayLibrary.Array_Length` _outactors)))

(fn `UserConstructionScript`)