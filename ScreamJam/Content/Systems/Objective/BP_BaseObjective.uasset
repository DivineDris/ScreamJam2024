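; BP_BaseObjective is a base objective actor that the player collects by interacting with it.
; On BeginPlay it looks up a BP_ObjectiveTrigger in the level and stores it as QuestTrigger.
; OnInteract proceeds only when the required-overlap flag and both player-overlap checks are true, then calls CollectObjective on the trigger and destroys itself.
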(event `self.ReceiveBeginPlay`
  (bind _returnvalue (`GameplayStatics.GetActorOfClass` "/Game/Systems/Objective/BP_ObjectiveTrigger.BP_ObjectiveTrigger_C"))
  (set `self.QuestTrigger` _returnvalue))

(event `/Game/Systems/Interaction/BPI_Interactable.OnInteract`
  (params (IsPlayerOverlapping :type Boolean))
  (if (`self.IsRequredPlayerOverlapping`)
    (if (and IsPlayerOverlapping (`self.IsOverlappingPlayer`))
      (`/Game/Systems/Objective/BPI_ObjectiveCollector.CollectObjective` (`self.QuestTrigger`))
      (`self.K2_DestroyActor`))))

(fn `UserConstructionScript`
  (`parent.UserConstructionScript`))