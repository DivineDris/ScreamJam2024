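; BP_InteractionCastRay finds the actor in front of the player camera, as a ray cast for interaction.
; CastTrace runs a Visibility line trace, behind a DoOnce, from the camera manager along its forward vector for Length, with debug drawing on.
; When the hit actor differs from TracedActor, it stores and returns the new one.
; BeginPlay and Tick are empty, so nothing in this Blueprint calls CastTrace.
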(event `self.ReceiveTick`
  (params (DeltaSeconds :type "Float (single-precision)")))

(fn `CastTrace`
  (returns (TracedActor :type "Actor Object Reference"))
  (bind _returnvalue (`GameplayStatics.GetPlayerCameraManager` 0))
  (bind _returnvalue_2 (`Actor.K2_GetActorLocation` _returnvalue))
  (`/Engine/EditorBlueprintResources/StandardMacros.DoOnce` false
    (:`Completed`
      (bind (_outhit _returnvalue_3) (`KismetSystemLibrary.LineTraceSingle` :`Start` _returnvalue_2 :`End` (+ _returnvalue_2 (* (`KismetMathLibrary.GetForwardVector` (`Actor.K2_GetActorRotation` _returnvalue)) (`self.Length`))) :`TraceChannel` "TraceTypeQuery1" :`DrawDebugType` "ForDuration"))
      (if _returnvalue_3
        (bind (_bblockinghit _binitialoverlap _time _distance _location _impactpoint _normal _impactnormal _physmat _hitactor) (`GameplayStatics.BreakHitResult` _outhit))
        (if (!= (`self.TracedActor`) _hitactor)
          (bind _output_get (set `self.TracedActor` _hitactor))
          (return _output_get))))))