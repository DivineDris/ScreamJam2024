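; Interactable outside door that swings open and closed and can send the player to another level.
; OnInteract checks player overlap flags, then prints a refusal if IsClosed is set.
; Otherwise a FlipFlop plays or reverses DoorTimeline to yaw DoorPivot, mirrored by IsReversed, with a DoOnce blocking retriggers until it finishes.
; The same interaction immediately opens the soft-referenced Level when IsReadyToLeave is set.
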(event `self.OnInteract`
  (params (IsPlayerOverlapping :type Boolean))
  (bind _level (`self.Level`))
  (if (`self.IsRequredPlayerOverlapping`)
    (if (and IsPlayerOverlapping (`self.IsOverlappingPlayer`))
      (if (`self.IsClosed`)
        (`KismetSystemLibrary.PrintString` "You can't go through that door" true true (struct :`R` 1.0 :`B` 0.006919 :`A` 1.0))
        (else
          (`|ExecutionSequence`
            (:`then_0`
              (`/Engine/EditorBlueprintResources/StandardMacros.DoOnce` false :!label _label
                (:`Completed`
                  (`/Engine/EditorBlueprintResources/StandardMacros.FlipFlop`
                    (:`A`
                      (bind (_direction _rotation) (`Timeline|DoorTimeline` :!via `PlayFromStart` :!label _label_2)
                        (:`Update`
                          (if (`self.IsReversed`)
                            (`SceneComponent.K2_SetRelativeRotation` (`self.DoorPivot`) (`KismetMathLibrary.MakeRotator` 0.0 0.0 (* _rotation -1.0)) false false)
                            (else
                              (`SceneComponent.K2_SetRelativeRotation` (`self.DoorPivot`) (`KismetMathLibrary.MakeRotator` 0.0 0.0 _rotation) false false))))
                        (:`Finished`
                          (goto _label :!via `Reset`))))
                    (:`B`
                      (goto _label_2 :!via `ReverseFromEnd`))))))
            (:`then_1`
              (if (`self.IsReadyToLeave`)
                (if (`KismetSystemLibrary.IsValidSoftObjectReference` _level)
                  (`GameplayStatics.OpenLevelBySoftObjectPtr` _level))))))))))

(fn `UserConstructionScript`)